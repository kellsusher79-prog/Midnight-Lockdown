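; BP_Turret is a stationary enemy that shoots at the player, and destroying the last one wins the game.
; A looping timer line-traces from FirePoint1 to the player and spawns an aimed BP_TurretProjectile when the trace hits the character.
; MLProjectile hits reduce health, scaled by the player's DamageMultiplier.
; At zero health it destroys itself; the last turret also plays the win sound and shows WBP_WinScreen with UI-only input.
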(event `OnActorHit_Event` :!signature `self.OnActorHit`
  (params (SelfActor :type "Actor Object Reference") (OtherActor :type "Actor Object Reference") (NormalImpulse :type "Vector Structure") (Hit :type "HitResult Structure (by ref)"))
  (bind _returnvalue (`GameplayStatics.GetPlayerController` 0))
  (cast `MLProjectile` OtherActor)
  (bind _asbp_first_person_character (cast `/Game/FirstPerson/Blueprints/BP_FirstPersonCharacter` (`GameplayStatics.GetPlayerCharacter` 0)))
  (bind _output_get (set `self.TurretHealth` (- (`self.TurretHealth`) (* (`/Game/FirstPerson/Blueprints/BP_FirstPersonCharacter.DamageMultiplier` _asbp_first_person_character) 25.0))))
  (if (<= _output_get 0.0)
    (bind _outactors (`GameplayStatics.GetAllActorsOfClass` "BP_Turret_C"))
    (if (<= (`KismetArrayLibrary.Array_Length` _outactors) 1)
      ; Winning Goal: Graphics
      (`GameplayStatics.PlaySound2D` "/Game/MidnightLockdown/Audio/A_SFX_Win.A_SFX_Win" 1.0 1.0 0.0 null null)
      (bind _returnvalue_2 (`|CreateWidget` "/Game/MidnightLockdown/UI/WBP_WinScreen.WBP_WinScreen_C"))
      (`UserWidget.AddToViewport` _returnvalue_2 0)
      (set `PlayerController.bShowMouseCursor` true _returnvalue)
      (`WidgetBlueprintLibrary.SetInputMode_UIOnlyEx` _returnvalue _returnvalue_2)
      (`self.K2_DestroyActor`)
      (else
        (`self.K2_DestroyActor`)))))

(event `self.ReceiveBeginPlay`
  (`|ExecutionSequence`
    (:`then_0`
      (`KismetSystemLibrary.K2_SetTimerDelegate` (delegate `TryFire`) 1.0 true))
    (:`then_1`
      (add `self.OnActorHit` (delegate `OnActorHit_Event`)))))

(event `TryFire`
  (bind _returnvalue (`self.K2_GetActorLocation` (`GameplayStatics.GetPlayerCharacter` 0)))
  (bind _returnvalue_2 (`SceneComponent.K2_GetComponentLocation` (`self.FirePoint1`)))
  (bind _outhit (`KismetSystemLibrary.LineTraceSingle` _returnvalue_2 _returnvalue "TraceTypeQuery1"))
  (cast `/Game/FirstPerson/Blueprints/BP_FirstPersonCharacter` (`.HitActor` (`GameplayStatics.BreakHitResult` _outhit)))
  (`|SpawnActorFromClass` "/Game/MidnightLockdown/Blueprints/BP_TurretProjectile.BP_TurretProjectile_C" (`KismetMathLibrary.MakeTransform` _returnvalue_2 (`KismetMathLibrary.FindLookAtRotation` _returnvalue_2 _returnvalue)) "AlwaysSpawn" "MultiplyWithRoot" null null))

(fn `UserConstructionScript`)